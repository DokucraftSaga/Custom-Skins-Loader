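; Tent decor actor that also bootstraps skin loading when it ticks in the main menu.
; Once the menu game mode is detected, it waits a second, then creates a UMG_SkinLoader widget if none exists.
; It adds the widget to the viewport, calls DumpSkins with an empty callback and reloads all skins.
; A separate helper draws a masked texture onto a render target, unused within these graphs.
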(event Custom|Nope
  (params (bSuccess :type Boolean)))

(event EventTick
  (params (DeltaSeconds :type Float%20%28single-precision%29))
  ;[1 1 1] Continue only if in the main menu
  (Utilities|Casting|CastToBP_MenuGameMode (Game|GetGameMode))
  (Utilities|FlowControl|DoOnce false
    (:Completed
      (Utilities|FlowControl|Delay 1.0)
      ;[1 1 1] Add the skin loader widget to the viewport if it isn't already there
      (bind _foundwidgets (Widget|GetAllWidgetsOfClass "/Game/UI/SkinLoader/UMG_SkinLoader.UMG_SkinLoader_C" true))
      (if (== (Utilities|Array|Length _foundwidgets) 0)
        (bind _returnvalue (UserInterface|CreateWidget "/Game/UI/SkinLoader/UMG_SkinLoader.UMG_SkinLoader_C"))
        (UserInterface|Viewport|AddtoViewport _returnvalue 0)
        (Default|DumpSkins _returnvalue (delegate Custom|Nope))
        (Default|ReloadAllSkins _returnvalue)))))

(fn ConstructionScript)